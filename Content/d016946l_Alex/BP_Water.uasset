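; BP_Water is a water hazard that puts out a burning BP_EscapeCharacter and electrocutes it if the water is electrified.
; Interface events set or clear the Electrified flag, which the Box checks only when overlap begins.
; Leaving the Box stops the character's electrocution.
; When BP_Electricity leaves, it only prints a debug message and does not clear the flag.
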(event `/Game/d016946l_Alex/Interfaces/BPI_ElementInteraction.I_electrifiedWater`
  (set `self.Electrified` true))

(event `/Game/d016946l_Alex/Interfaces/BPI_ElementInteraction.I_notElectrified`
  (set `self.Electrified` false))

(event `self.Box.OnComponentBeginOverlap`
  (params (OverlappedComponent :type "PrimitiveComponent Object Reference") (OtherActor :type "Actor Object Reference") (OtherComp :type "PrimitiveComponent Object Reference") (OtherBodyIndex :type Integer) (bFromSweep :type Boolean) (SweepResult :type "HitResult Structure (by ref)"))
  ;[1 1 1] If player touches water and is on fire, stop the fire
  (bind _asbp_escape_character (cast `/Game/s020301l/BP_EscapeCharacter` OtherActor))
  (`|ExecutionSequence`
    (:`then_0`
      (if (`/Game/s020301l/BP_EscapeCharacter.PlayerOnFire?` _asbp_escape_character)
        (`/Game/s020301l/BP_EscapeCharacter.StopBurning` _asbp_escape_character)))
    (:`then_1`
      (if (`self.Electrified`)
        (message `/Game/d016946l_Alex/Interfaces/BPI_ElementInteraction.I_Electrocute` _asbp_escape_character)
        (`KismetSystemLibrary.PrintString` "damaging player")))))

(event `self.Box.OnComponentEndOverlap`
  (params (OverlappedComponent :type "PrimitiveComponent Object Reference") (OtherActor :type "Actor Object Reference") (OtherComp :type "PrimitiveComponent Object Reference") (OtherBodyIndex :type Integer))
  ;[1 1 1] Checks if  Electricity left water and stop electrifying it
  (`|ExecutionSequence`
    (:`then_0`
      (cast `/Game/d016946l_Alex/BP_Electricity` OtherActor)
      (`KismetSystemLibrary.PrintString` "no longer electrified"))
    (:`then_1`
      (bind _asbp_escape_character (cast `/Game/s020301l/BP_EscapeCharacter` OtherActor))
      (`/Game/s020301l/BP_EscapeCharacter.StopElectrocution` _asbp_escape_character))))

(fn `UserConstructionScript`)