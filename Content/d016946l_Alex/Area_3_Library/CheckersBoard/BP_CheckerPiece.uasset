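; Checker piece for the library area's checkers board that snaps to a chosen square and tracks overlaps in four directions.
; The construction script applies its material and, if flagged attached, snaps it to one of the board's 64 square components by one-based slot index.
; Left, Right, Front and Back overlap events store their own OverlappedComponent, not the other component, and its display name as that direction's move.
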(event `self.Left.OnComponentBeginOverlap`
  (params (OverlappedComponent :type "PrimitiveComponent Object Reference") (OtherActor :type "Actor Object Reference") (OtherComp :type "PrimitiveComponent Object Reference") (OtherBodyIndex :type Integer) (bFromSweep :type Boolean) (SweepResult :type "HitResult Structure (by ref)"))
  (set `self.LeftMove` OverlappedComponent)
  (set `self.LeftBoxName` (`KismetSystemLibrary.GetDisplayName` OverlappedComponent)))

(event `self.Right.OnComponentBeginOverlap`
  (params (OverlappedComponent :type "PrimitiveComponent Object Reference") (OtherActor :type "Actor Object Reference") (OtherComp :type "PrimitiveComponent Object Reference") (OtherBodyIndex :type Integer) (bFromSweep :type Boolean) (SweepResult :type "HitResult Structure (by ref)"))
  (set `self.RightMove` OverlappedComponent)
  (set `self.RightBoxName` (`KismetSystemLibrary.GetDisplayName` OverlappedComponent)))

(event `self.Back.OnComponentBeginOverlap`
  (params (OverlappedComponent :type "PrimitiveComponent Object Reference") (OtherActor :type "Actor Object Reference") (OtherComp :type "PrimitiveComponent Object Reference") (OtherBodyIndex :type Integer) (bFromSweep :type Boolean) (SweepResult :type "HitResult Structure (by ref)"))
  (set `self.BackMove` OverlappedComponent)
  (set `self.BackBoxName` (`KismetSystemLibrary.GetDisplayName` OverlappedComponent)))

(event `self.Front.OnComponentBeginOverlap`
  (params (OverlappedComponent :type "PrimitiveComponent Object Reference") (OtherActor :type "Actor Object Reference") (OtherComp :type "PrimitiveComponent Object Reference") (OtherBodyIndex :type Integer) (bFromSweep :type Boolean) (SweepResult :type "HitResult Structure (by ref)"))
  (set `self.FrontMove` OverlappedComponent)
  (set `self.FrontBoxName` (`KismetSystemLibrary.GetDisplayName` OverlappedComponent)))

(fn `UserConstructionScript`
  (bind _checkerboard_ref (`self.CheckerBoard_ref`))
  (`PrimitiveComponent.SetMaterial` (`self.PieceMesh`) 0 (`self.Material`))
  (if (`self.IsAttached?`)
    (`self.K2_AttachToComponent` (`|GetArrayItem` (`|MakeArray` (`/Game/d016946l_Alex/Area_3_Library/CheckersBoard/P_CheckersBoard.a1b` _checkerboard_ref) (`/Game/d016946l_Alex/Area_3_Library/CheckersBoard/P_CheckersBoard.a2b` _checkerboard_ref) (`/Game/d016946l_Alex/Area_3_Library/CheckersBoard/P_CheckersBoard.a3b` _checkerboard_ref) (`/Game/d016946l_Alex/Area_3_Library/CheckersBoard/P_CheckersBoard.a4b` _checkerboard_ref) (`/Game/d016946l_Alex/Area_3_Library/CheckersBoard/P_CheckersBoard.a5b` _checkerboard_ref) (`/Game/d016946l_Alex/Area_3_Library/CheckersBoard/P_CheckersBoard.a6b` _checkerboard_ref) (`/Game/d016946l_Alex/Area_3_Library/CheckersBoard/P_CheckersBoard.a7b` _checkerboard_ref) (`/Game/d016946l_Alex/Area_3_Library/CheckersBoard/P_CheckersBoard.a8b` _checkerboard_ref) (`/Game/d016946l_Alex/Area_3_Library/CheckersBoard/P_CheckersBoard.b1b` _checkerboard_ref) (`/Game/d016946l_Alex/Area_3_Library/CheckersBoard/P_CheckersBoard.b2b` _checkerboard_ref) (`/Game/d016946l_Alex/Area_3_Library/CheckersBoard/P_CheckersBoard.b3b` _checkerboard_ref) (`/Game/d016946l_Alex/Area_3_Library/CheckersBoard/P_CheckersBoard.b4b` _checkerboard_ref) (`/Game/d016946l_Alex/Area_3_Library/CheckersBoard/P_CheckersBoard.b5b` _checkerboard_ref) (`/Game/d016946l_Alex/Area_3_Library/CheckersBoard/P_CheckersBoard.b6b` _checkerboard_ref) (`/Game/d016946l_Alex/Area_3_Library/CheckersBoard/P_CheckersBoard.b7b` _checkerboard_ref) (`/Game/d016946l_Alex/Area_3_Library/CheckersBoard/P_CheckersBoard.b8b` _checkerboard_ref) (`/Game/d016946l_Alex/Area_3_Library/CheckersBoard/P_CheckersBoard.c1b` _checkerboard_ref) (`/Game/d016946l_Alex/Area_3_Library/CheckersBoard/P_CheckersBoard.c2b` _checkerboard_ref) (`/Game/d016946l_Alex/Area_3_Library/CheckersBoard/P_CheckersBoard.c3b` _checkerboard_ref) (`/Game/d016946l_Alex/Area_3_Library/CheckersBoard/P_CheckersBoard.c4b` _checkerboard_ref) (`/Game/d016946l_Alex/Area_3_Library/CheckersBoard/P_CheckersBoard.c5b` _checkerboard_ref) (`/Game/d016946l_Alex/Area_3_Library/CheckersBoard/P_CheckersBoard.c6b` _checkerboard_ref) (`/Game/d016946l_Alex/Area_3_Library/CheckersBoard/P_CheckersBoard.c7b` _checkerboard_ref) (`/Game/d016946l_Alex/Area_3_Library/CheckersBoard/P_CheckersBoard.c8b` _checkerboard_ref) (`/Game/d016946l_Alex/Area_3_Library/CheckersBoard/P_CheckersBoard.d1b` _checkerboard_ref) (`/Game/d016946l_Alex/Area_3_Library/CheckersBoard/P_CheckersBoard.d2b` _checkerboard_ref) (`/Game/d016946l_Alex/Area_3_Library/CheckersBoard/P_CheckersBoard.d3b` _checkerboard_ref) (`/Game/d016946l_Alex/Area_3_Library/CheckersBoard/P_CheckersBoard.d4b` _checkerboard_ref) (`/Game/d016946l_Alex/Area_3_Library/CheckersBoard/P_CheckersBoard.d5b` _checkerboard_ref) (`/Game/d016946l_Alex/Area_3_Library/CheckersBoard/P_CheckersBoard.d6b` _checkerboard_ref) (`/Game/d016946l_Alex/Area_3_Library/CheckersBoard/P_CheckersBoard.d7b` _checkerboard_ref) (`/Game/d016946l_Alex/Area_3_Library/CheckersBoard/P_CheckersBoard.d8b` _checkerboard_ref) (`/Game/d016946l_Alex/Area_3_Library/CheckersBoard/P_CheckersBoard.e1b` _checkerboard_ref) (`/Game/d016946l_Alex/Area_3_Library/CheckersBoard/P_CheckersBoard.e2b` _checkerboard_ref) (`/Game/d016946l_Alex/Area_3_Library/CheckersBoard/P_CheckersBoard.e3b` _checkerboard_ref) (`/Game/d016946l_Alex/Area_3_Library/CheckersBoard/P_CheckersBoard.e4b` _checkerboard_ref) (`/Game/d016946l_Alex/Area_3_Library/CheckersBoard/P_CheckersBoard.e5b` _checkerboard_ref) (`/Game/d016946l_Alex/Area_3_Library/CheckersBoard/P_CheckersBoard.e6b` _checkerboard_ref) (`/Game/d016946l_Alex/Area_3_Library/CheckersBoard/P_CheckersBoard.e7b` _checkerboard_ref) (`/Game/d016946l_Alex/Area_3_Library/CheckersBoard/P_CheckersBoard.e8b` _checkerboard_ref) (`/Game/d016946l_Alex/Area_3_Library/CheckersBoard/P_CheckersBoard.f1b` _checkerboard_ref) (`/Game/d016946l_Alex/Area_3_Library/CheckersBoard/P_CheckersBoard.f2b` _checkerboard_ref) (`/Game/d016946l_Alex/Area_3_Library/CheckersBoard/P_CheckersBoard.f3b` _checkerboard_ref) (`/Game/d016946l_Alex/Area_3_Library/CheckersBoard/P_CheckersBoard.f4b` _checkerboard_ref) (`/Game/d016946l_Alex/Area_3_Library/CheckersBoard/P_CheckersBoard.f5b` _checkerboard_ref) (`/Game/d016946l_Alex/Area_3_Library/CheckersBoard/P_CheckersBoard.f6b` _checkerboard_ref) (`/Game/d016946l_Alex/Area_3_Library/CheckersBoard/P_CheckersBoard.f7b` _checkerboard_ref) (`/Game/d016946l_Alex/Area_3_Library/CheckersBoard/P_CheckersBoard.f8b` _checkerboard_ref) (`/Game/d016946l_Alex/Area_3_Library/CheckersBoard/P_CheckersBoard.g1b` _checkerboard_ref) (`/Game/d016946l_Alex/Area_3_Library/CheckersBoard/P_CheckersBoard.g2b` _checkerboard_ref) (`/Game/d016946l_Alex/Area_3_Library/CheckersBoard/P_CheckersBoard.g3b` _checkerboard_ref) (`/Game/d016946l_Alex/Area_3_Library/CheckersBoard/P_CheckersBoard.g4b` _checkerboard_ref) (`/Game/d016946l_Alex/Area_3_Library/CheckersBoard/P_CheckersBoard.g5b` _checkerboard_ref) (`/Game/d016946l_Alex/Area_3_Library/CheckersBoard/P_CheckersBoard.g6b` _checkerboard_ref) (`/Game/d016946l_Alex/Area_3_Library/CheckersBoard/P_CheckersBoard.g7b` _checkerboard_ref) (`/Game/d016946l_Alex/Area_3_Library/CheckersBoard/P_CheckersBoard.g8b` _checkerboard_ref) (`/Game/d016946l_Alex/Area_3_Library/CheckersBoard/P_CheckersBoard.h1b` _checkerboard_ref) (`/Game/d016946l_Alex/Area_3_Library/CheckersBoard/P_CheckersBoard.h2b` _checkerboard_ref) (`/Game/d016946l_Alex/Area_3_Library/CheckersBoard/P_CheckersBoard.h3b` _checkerboard_ref) (`/Game/d016946l_Alex/Area_3_Library/CheckersBoard/P_CheckersBoard.h4b` _checkerboard_ref) (`/Game/d016946l_Alex/Area_3_Library/CheckersBoard/P_CheckersBoard.h5b` _checkerboard_ref) (`/Game/d016946l_Alex/Area_3_Library/CheckersBoard/P_CheckersBoard.h6b` _checkerboard_ref) (`/Game/d016946l_Alex/Area_3_Library/CheckersBoard/P_CheckersBoard.h7b` _checkerboard_ref) (`/Game/d016946l_Alex/Area_3_Library/CheckersBoard/P_CheckersBoard.h8b` _checkerboard_ref)) (- (`self.slot to attach to`) 1)) "None" "SnapToTarget" "KeepWorld" "KeepWorld")))