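; BP_Student_Screen is a student computer screen in the computer room area that can be switched on and off.
; TurnOnScreens sets the number text, applies the on-screen material to the mesh, opens the media source and shows both text and mesh.
; TurnOffScreens closes the media and hides both components.
; The file contains no trigger logic, only these two events and an empty construction script.
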(event `Turn On Screens`
  (`|ExecutionSequence`
    (:`then_0`
      (`TextRenderComponent.K2_SetText` (`self.TextRender`) (`self.TextNumber`))
      (`PrimitiveComponent.SetMaterial` (`self.StaticMeshComponent`) 0 (`self.OnScreenMaterial`)))
    (:`then_2`
      (`MediaPlayer.OpenSource` (`self.Target`) (`self.Media Source`)))
    (:`then_3`
      (`SceneComponent.SetVisibility` (`self.TextRender`) true false))
    (:`then_4`
      (`SceneComponent.SetVisibility` (`self.StaticMeshComponent`) true false))))

(event `Turn Off Screens`
  (`|ExecutionSequence`
    (:`then_0`
      (`MediaPlayer.Close` (`self.Target`)))
    (:`then_1`
      (`SceneComponent.SetVisibility` (`self.TextRender`) false false))
    (:`then_2`
      (`SceneComponent.SetVisibility` (`self.StaticMeshComponent`) false false))))

(fn `UserConstructionScript`)