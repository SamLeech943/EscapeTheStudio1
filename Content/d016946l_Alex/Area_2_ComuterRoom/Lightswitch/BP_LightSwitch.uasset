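; BP_LightSwitch is an interactable light switch that toggles a set of lights and light boxes on and off.
; On the IInteract event, two FlipFlops alternate between on and off, starting with on.
; One sets the point light intensity of every BP_Light in the editor-assigned LightRef array.
; The other swaps the mesh material on each LightBoxRef entry between lit and black transparent.
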(event `/Game/c013265l/Interfaces/BPI_Interaction.I_Interact`
  (params (InteractingCharacter :type "/Game/s020301l/Blueprints/Character/BP_EscapeCharacter Object Reference") (InteractingWirePawn :type "/Game/c013265l/Puzzles/PCRoom/Blueprints/P_WirePuzzle Object Reference"))
  (bind _lightbox_ref (`self.LightBox_ref`))
  (bind _light_ref (`self.Light_ref`))
  (`KismetSystemLibrary.PrintString` "switch")
  (`|ExecutionSequence`
    (:`then_0`
      ;[1 1 1] This LightSwitch is dynamic. Can be used for any light that is the BP_Light in my folder, it's an array so from the editor select with an eye drop what light you want to switch
      (`/Engine/EditorBlueprintResources/StandardMacros.FlipFlop`
        (:`A`
          (for _array_element _light_ref
            (`LightComponent.SetIntensity` (`/Game/d016946l_Alex/BP_Light.PointLight` _array_element) 1000.0)))
        (:`B`
          (for _array_element_2 _light_ref
            (`LightComponent.SetIntensity` (`/Game/d016946l_Alex/BP_Light.PointLight` _array_element_2) 0.0)))))
    (:`then_1`
      (`/Engine/EditorBlueprintResources/StandardMacros.FlipFlop`
        (:`A`
          (for _array_element_3 _lightbox_ref
            (`PrimitiveComponent.SetMaterial` (`StaticMeshActor.StaticMeshComponent` _array_element_3) 0 "/Game/d016946l_Alex/Area_2_ComuterRoom/Lightswitch/M_LightBox_Light.M_LightBox_Light")))
        (:`B`
          (for _array_element_4 _lightbox_ref
            (`PrimitiveComponent.SetMaterial` (`StaticMeshActor.StaticMeshComponent` _array_element_4) 0 "/Game/d016946l_Alex/Area_2_ComuterRoom/Lightswitch/M_LightBox_BlackTrasparent.M_LightBox_BlackTrasparent")))))))

(fn `UserConstructionScript`)