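; BP_Gregg is a watcher NPC with look-around and read-book states, meant to spot BP_EscapeCharacter.
; LookAround enables collision and turns it 90 degrees by timeline; ReadBook disables collision and stops the turn.
; BeginPlay sets one-shot timers for both, though LookAround's zero delay means it never fires.
; Capsule overlap draws a visibility trace from the Sphere to the player, printing detection if nothing blocks it.
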(event `self.ReceiveBeginPlay`
  (`KismetSystemLibrary.K2_SetTimerDelegate` (delegate `LookAround`))
  (`KismetSystemLibrary.K2_SetTimerDelegate` (delegate `ReadBook`) 8.0))

(event `LookAround`
  (bind _initialrotation (`self.InitialRotation`))
  (`self.SetActorEnableCollision` true)
  (set `self.InitialRotation` (`self.K2_GetActorRotation`))
  (bind (_direction _newtrack_0) (`Timeline|Timeline_0` :!label _label)
    (:`Update`
      (`self.K2_SetActorRotation` (`KismetMathLibrary.RLerp` _initialrotation (`KismetMathLibrary.ComposeRotators` _initialrotation (struct :`Yaw` 90.0)) _newtrack_0)))
    (:`Finished`
      (`self.ReadBook`))))

(event `ReadBook`
  (`self.SetActorEnableCollision` false)
  (goto _label :!via `Stop`))

(event `self.Capsule.OnComponentBeginOverlap`
  (params (OverlappedComponent :type "PrimitiveComponent Object Reference") (OtherActor :type "Actor Object Reference") (OtherComp :type "PrimitiveComponent Object Reference") (OtherBodyIndex :type Integer) (bFromSweep :type Boolean) (SweepResult :type "HitResult Structure (by ref)"))
  (bind _asbp_escape_character (cast `/Game/UserWork/s020301l/Blueprints/Character/BP_EscapeCharacter` OtherActor))
  (bind _outhit (`KismetSystemLibrary.LineTraceSingle` :`Start` (`SceneComponent.K2_GetComponentLocation` (`self.Sphere`)) :`End` (`self.K2_GetActorLocation` _asbp_escape_character) :`TraceChannel` "TraceTypeQuery1" :`DrawDebugType` "Persistent"))
  (`KismetSystemLibrary.PrintString` "Searching")
  (if (not (`GameplayStatics.BreakHitResult` _outhit))
    (`KismetSystemLibrary.PrintString` "I found you")))

(fn `UserConstructionScript`)