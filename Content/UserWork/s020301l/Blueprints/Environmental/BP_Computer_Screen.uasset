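; BP_Computer_Screen is an environmental computer display with left and right screens, each switchable between off and on.
; BeginPlay starts it powered off and copies DisplayText into both text renders.
; PowerOff applies a black material and hides the text, while PowerOn applies DisplayMaterial to both screens and shows the text.
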(event `self.ReceiveBeginPlay`
  (bind _display_text (`self.Display Text`))
  (`self.PowerOff`)
  (`TextRenderComponent.K2_SetText` (`self.TextRender`) _display_text)
  (`TextRenderComponent.K2_SetText` (`self.TextRender1`) _display_text))

(event `PowerOff`
  (`PrimitiveComponent.SetMaterial` (`self.Screen_Right`) 0 "/Game/UserWork/s020301l/Materials/M_Black.M_Black")
  (`PrimitiveComponent.SetMaterial` (`self.Screen_Left`) 0 "/Game/UserWork/s020301l/Materials/M_Black.M_Black")
  (`SceneComponent.SetVisibility` (`self.TextRender`) false false)
  (`SceneComponent.SetVisibility` (`self.TextRender1`) false false))

(event `PowerOn`
  (bind _display_material (`self.Display Material`))
  (`PrimitiveComponent.SetMaterial` (`self.Screen_Right`) 0 _display_material)
  (`PrimitiveComponent.SetMaterial` (`self.Screen_Left`) 0 _display_material)
  (`SceneComponent.SetVisibility` (`self.TextRender`) true false)
  (`SceneComponent.SetVisibility` (`self.TextRender1`) true false))

(fn `UserConstructionScript`)