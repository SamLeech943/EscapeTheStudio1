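; An interactable, lockable door whose indicator light shows red when locked and green when unlocked.
; SetLocked stores the state and reruns the BeginPlay light check, which also plays the door-open sound whenever the door is unlocked.
; Interacting while unlocked alternates a timeline forward and back to rotate the door mesh's yaw.
; OpenDoor and CloseDoor drive that timeline directly, ignoring the lock, with a knob sound on close.
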(event `SetLocked`
  (params (`IsLocked?` :type Boolean))
  (set `self.locked` `IsLocked?`)
  (`self.ChangeMaterial`))

(event `self.ReceiveBeginPlay`
  (bind _doorlight (`self.DoorLight`))
  ;[1 1 1] At the beginning of the game it checks if the door is locked and sets the light properly
  (if (`self.locked`) :!label _label
    (`PrimitiveComponent.SetMaterial` _doorlight 0 "/Game/UserWork/d016946l_Alex/Area_2_ComuterRoom/Lightswitch_NOT_USED/M_LightBox_RedEmergency.M_LightBox_RedEmergency")
    (else
      (`PrimitiveComponent.SetMaterial` _doorlight 0 "/Game/UserWork/s020301l/Materials/M_GreenEmissive.M_GreenEmissive")
      (`GameplayStatics.PlaySound2D` "/Game/UserWork/l014519/Audio/Door_Open/DoorOpen.DoorOpen" 1.0 1.0 0.0 null null))))

(event `ChangeMaterial`
  ;[1 1 1] At the beginning of the game it checks if the door is locked and sets the light properly
  (goto _label))

(event `/Game/UserWork/c013265l/Interfaces/BPI_Interaction.I_Interact`
  (params (InteractingCharacter :type "/Game/UserWork/s020301l/Blueprints/Character/BP_EscapeCharacter Object Reference") (InteractingWirePawn :type "/Game/UserWork/c013265l/Puzzles/PCRoom/Blueprints/P_WirePuzzle Object Reference"))
  (if (not (`self.locked`))
    (`/Engine/EditorBlueprintResources/StandardMacros.FlipFlop`
      (:`A`
        (bind (_direction _newtrack_0) (`Timeline|Timeline_0` :!label _label_2)
          (:`Update`
            (`SceneComponent.K2_SetRelativeRotation` (`self.Cube5`) (`KismetMathLibrary.MakeRotator` 0.0 0.0 _newtrack_0) false false))))
      (:`B`
        (goto _label_2 :!via `Reverse`)))))

(event `OpenDoor`
  (goto _label_2))

(event `CloseDoor`
  (`GameplayStatics.PlaySound2D` "/Game/UserWork/l014519/Audio/Door_Close/PM_HD_Source_99_Door__Knob__Twist__Turn.PM_HD_Source_99_Door__Knob__Twist__Turn" 1.0 1.0 0.0 null null)
  (goto _label_2 :!via `Reverse`))

(fn `UserConstructionScript`)