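; BP_Student_Screen is a computer-room screen that can be switched on and off through two custom events.
; TurnOnScreens applies the desktop material, sets the text number, shows it only if TextOnScreen is set, and reveals the mesh.
; It also opens a media source when a valid player is assigned, for screens with video.
; TurnOffScreens closes that media, hides the text and swaps the screen to a black material.
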(event `Turn On Screens`
  (bind _target (`self.Target`))
  (bind _textrender (`self.TextRender`))
  ;[1 1 1] Turn on screen function will set: the dekstop background of the screens, text number, and a video if it has one (this is for you oliver)
  (`|ExecutionSequence`
    (:`then_0`
      (`TextRenderComponent.K2_SetText` (`self.TextRender`) (`self.TextNumber`)))
    (:`then_1`
      (`PrimitiveComponent.SetMaterial` (`self.StaticMeshComponent`) 0 (`self.OnScreenMaterial`)))
    (:`then_2`
      (`/Engine/EditorBlueprintResources/StandardMacros.IsValid` _target
        (:`Is Valid`
          (`MediaPlayer.OpenSource` _target (`self.Media Source`)))))
    (:`then_3`
      (if (`self.TextOnScreen?`)
        (`SceneComponent.SetVisibility` _textrender true false)
        (else
          (`SceneComponent.SetVisibility` _textrender false false))))
    (:`then_4`
      (`SceneComponent.SetVisibility` (`self.StaticMeshComponent`) true false))))

(event `Turn Off Screens`
  (bind _target (`self.Target`))
  ;[1 1 1] turn off screen function is called to delete everything that was happening on them and set the screen to a black material
  (`|ExecutionSequence`
    (:`then_0`
      (`/Engine/EditorBlueprintResources/StandardMacros.IsValid` _target
        (:`Is Valid`
          (`MediaPlayer.Close` _target))))
    (:`then_1`
      (`SceneComponent.SetVisibility` (`self.TextRender`) false false))
    (:`then_2`
      (`PrimitiveComponent.SetMaterial` (`self.StaticMeshComponent`) 0 "/Game/UserWork/d016946l_Alex/Area_2_ComuterRoom/Clues/M_Black.M_Black"))))

(fn `UserConstructionScript`)