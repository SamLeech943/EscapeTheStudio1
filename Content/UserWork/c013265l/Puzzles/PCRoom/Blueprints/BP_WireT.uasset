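; BP_WireT is a wire piece for the PC Room puzzle that relays voltage to a connected neighbor.
; On a wire-connected interface event, it adds its charge modifier to the incoming charge to set its current voltage.
; It then scans overlapping components tagged Connector, skipping the sender, and passes the voltage and itself to the owner.
; A DoOnce limits forwarding to the first match per signal and resets after the loop.
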(event `/Game/UserWork/c013265l/Interfaces/BPI_WirePuzzle.I_WireConnected`
  (params (ChargetoAdd :type Integer) (WiretoIgnore :type "Actor Object Reference"))
  (set `self.Wireto Ignore` WiretoIgnore)
  (set `self.CurrentVoltage` (+ ChargetoAdd (`self.WireChargeMod`)))
  (for _array_element (`self.GetOverlappingComponents`)
    (if (`ActorComponent.ComponentHasTag` _array_element "Connector")
      (bind _returnvalue (`ActorComponent.GetOwner` _array_element))
      (if (!= _returnvalue (`self.Wireto Ignore`))
        (`/Engine/EditorBlueprintResources/StandardMacros.DoOnce` false :!label _label
          (:`Completed`
            (message `/Game/UserWork/c013265l/Interfaces/BPI_WirePuzzle.I_WireConnected` _returnvalue (`self.CurrentVoltage`) self))))))
  (goto _label :!via `Reset`))

(fn `UserConstructionScript`
  (`parent.UserConstructionScript`))