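; Interactable wall clock puzzle where the player turns the hands to bring the short hand onto a target.
; Interacting enables input; holding Q or E plays or reverses the RotateHandles timeline, turning the short hand at one-twelfth the long hand's rate.
; ShortHandBox overlapping TargetBox currently only prints "win".
; An older timer-based rotation (StartRotating, HandleRotation) remains but nothing calls it.
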(event `/Game/UserWork/c013265l/Interfaces/BPI_Interaction.I_CanInteractWithObject`
  (params (InteractingChar :type "Pawn Object Reference"))
  (set `self.Interacting Char` InteractingChar)
  (`self.EnableInput` (`GameplayStatics.GetPlayerController` 0)))

(event `/Game/UserWork/c013265l/Interfaces/BPI_Interaction.I_StopInteractWithObject`
  (set `self.Interacting Char` null)
  (`self.DisableInput` (`GameplayStatics.GetPlayerController` 0))
  (`self.StopRotating`))

(event `Key|Q`
  (params (Key :type "Key Structure"))
  ;[0.01304 0.2812 0.05831] c013265l - Rotate Handles
  (:`Pressed`
    (bind (_direction _rottoadd) (`Timeline|RotateHandles` :!label _label)
      (:`Update`
        (switch `ETimelineDirection` _direction
          (:`Forward`
            (`SceneComponent.K2_AddLocalRotation` (`self.wallclockLongHand`) (`KismetMathLibrary.MakeRotator` 0.0 _rottoadd) false false)
            (`SceneComponent.K2_AddLocalRotation` (`self.wallclockShortHand`) (`KismetMathLibrary.MakeRotator` 0.0 (/ _rottoadd 12.0)) false false))
          (:`Backward`
            (bind _returnvalue (* _rottoadd -1.0))
            (`SceneComponent.K2_AddLocalRotation` (`self.wallclockLongHand`) (`KismetMathLibrary.MakeRotator` 0.0 _returnvalue) false false)
            (`SceneComponent.K2_AddLocalRotation` (`self.wallclockShortHand`) (`KismetMathLibrary.MakeRotator` 0.0 (/ _returnvalue 12.0)) false false))))))
  (:`Released`
    (goto _label :!via `Stop`)))

(event `Key|E`
  (params (Key :type "Key Structure"))
  ;[0.01304 0.2812 0.05831] c013265l - Rotate Handles
  (:`Pressed`
    (goto _label :!via `Reverse`))
  (:`Released`
    (goto _label :!via `Stop`)))

(event `StopRotating`
  ;[0.01304 0.2812 0.05831] c013265l - Rotate Handles
  (goto _label :!via `Stop`))

(event `StartRotating`
  (params (Clockwise :type Boolean))
  (bind _returnvalue (`KismetSystemLibrary.K2_SetTimerDelegate` (delegate `HandleRotation`) 0.1 true))
  (set `self.HandleRotHandle` _returnvalue))

(event `HandleRotation`
  (if (stale `StartRotating` Clockwise)
    (`SceneComponent.K2_AddRelativeRotation` (`self.wallclockLongHand`) (`KismetMathLibrary.MakeRotator` 3.0) false false)
    (`SceneComponent.K2_AddRelativeRotation` (`self.wallclockShortHand`) (`KismetMathLibrary.MakeRotator` 0.6) false false)
    (else
      (`SceneComponent.K2_AddRelativeRotation` (`self.wallclockLongHand`) (`KismetMathLibrary.MakeRotator` -3.0) false false)
      (`SceneComponent.K2_AddRelativeRotation` (`self.wallclockShortHand`) (`KismetMathLibrary.MakeRotator` -0.6) false false))))

(event `self.ShortHandBox.OnComponentBeginOverlap`
  (params (OverlappedComponent :type "PrimitiveComponent Object Reference") (OtherActor :type "Actor Object Reference") (OtherComp :type "PrimitiveComponent Object Reference") (OtherBodyIndex :type Integer) (bFromSweep :type Boolean) (SweepResult :type "HitResult Structure (by ref)"))
  ;[0.01304 0.2812 0.05831] c013265l - On PuzzleComplete
  (if (== OtherComp (`self.TargetBox`))
    (`KismetSystemLibrary.PrintString` "win")))

(fn `UserConstructionScript`)