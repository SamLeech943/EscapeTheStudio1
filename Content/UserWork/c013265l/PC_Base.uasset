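; Player controller for an escape-room style first-person game that routes interaction, item handling and mouse input to BP_EscapeCharacter and the held item.
; It creates the Player_UI widget, line-traces from the camera for BPI_Interaction actors, and relays drop, inspect and attach actions through interface messages.
; Interface events track the held item, toggle crosshair and input, and run a looping timer that sends deprojected mouse positions to the pawn.
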(event `self.ReceiveBeginPlay`
  (bind _asbp_escape_character (cast `/Game/s020301l/Blueprints/Character/BP_EscapeCharacter` (`self.K2_GetPawn`)))
  (set `self.InteractingChar` _asbp_escape_character)
  (bind _returnvalue (`|CreateWidget` "/Game/A018745l/UI/Player_UI.Player_UI_C" self))
  (bind _output_get (set `self.Player UI` _returnvalue))
  (`UserWidget.AddToViewport` _output_get 0)
  (message `/Game/UserWork/c013265l/Interfaces/BPI_Interaction.I_PlayerUIReferencer` (`self.K2_GetPawn` (`GameplayStatics.GetPlayerController` 0)) (`self.Player UI`)))

(event `InputAction|Interact`
  (params (Key :type "Key Structure"))
  (bind _interactingchar (`self.InteractingChar`))
  (bind _firstpersoncamera (`/Game/s020301l/Blueprints/Character/BP_EscapeCharacter.FirstPersonCamera` (`self.InteractingChar`)))
  (bind _returnvalue (`SceneComponent.K2_GetComponentLocation` _firstpersoncamera))
  (:`Pressed`
    (message `/Game/UserWork/c013265l/Interfaces/BPI_Interaction.I_UiInteract` _interactingchar Key)
    (if (not (`self.HasItem`))
      (bind (_outhit _returnvalue_2) (`KismetSystemLibrary.LineTraceSingleForObjects` _returnvalue (+ _returnvalue (* (`KismetMathLibrary.GetForwardVector` (`SceneComponent.K2_GetComponentRotation` _firstpersoncamera)) 500.0)) (`|MakeArray` "ObjectTypeQuery8" :!type "EObjectTypeQuery Enum")))
      (if _returnvalue_2
        (bind (_bblockinghit _binitialoverlap _time _distance _location _impactpoint _normal _impactnormal _physmat _hitactor) (`GameplayStatics.BreakHitResult` _outhit))
        (if (`KismetSystemLibrary.DoesImplementInterface` _hitactor "/Game/UserWork/c013265l/Interfaces/BPI_Interaction.BPI_Interaction_C")
          (bind _output_get (set `self.HeldItem` _hitactor))
          (message `/Game/UserWork/c013265l/Interfaces/BPI_Interaction.I_Interact` _output_get (`self.InteractingChar`) null)
          (set `self.IsInspecting` false)))))
  (:`Released`
    (message `/Game/UserWork/c013265l/Interfaces/BPI_Interaction.I_ReleaseUIClick` _interactingchar)))

(event `/Game/UserWork/c013265l/Interfaces/BPI_Interaction.I_IsDropped`
  (set `self.HasItem` false)
  (`Widget.SetVisibility` (`/Game/A018745l/UI/Player_UI.Crosshair` (`self.Player UI`)) "Visible"))

(event `/Game/UserWork/c013265l/Interfaces/BPI_WirePuzzle.I_StartTrackingMouse`
  (bind _returnvalue (`KismetSystemLibrary.K2_SetTimerDelegate` (delegate `TrackingMouse`) 0.005 true))
  (set `self.MouseTrackerHandle` _returnvalue))

(event `/Game/UserWork/c013265l/Interfaces/BPI_Interaction.I_IsPickedUp`
  (set `self.HasItem` true)
  (`Widget.SetVisibility` (`/Game/A018745l/UI/Player_UI.Crosshair` (`self.Player UI`)) "Hidden")
  (`Widget.SetVisibility` (`/Game/A018745l/UI/Player_UI.GrabIcon` (`self.Player UI`)) "Hidden"))

(event `InputAction|DropItem`
  (params (Key :type "Key Structure"))
  (:`Pressed`
    (if (`self.Should Freeze`)
      _
      (elif (`self.HasItem`)
        (message `/Game/UserWork/c013265l/Interfaces/BPI_Interaction.I_DropItem` (`self.HeldItem`) (`self.InteractingChar`))))))

(event `TrackingMouse`
  (`self.GetCurrentMousePosition`))

(event `/Game/UserWork/c013265l/Interfaces/BPI_WirePuzzle.I_StopTrackingMouse`
  (`KismetSystemLibrary.K2_ClearAndInvalidateTimerHandle` (`self.MouseTrackerHandle`)))

(event `InputAction|Inspect`
  (params (Key :type "Key Structure"))
  (bind _helditem (`self.HeldItem`))
  (:`Pressed`
    (if (`self.HasItem`)
      (if (`self.IsInspecting`)
        (set `self.IsInspecting` false)
        (message `/Game/UserWork/c013265l/Interfaces/BPI_Interaction.I_StopInspecting` _helditem)
        (else
          (set `self.IsInspecting` true)
          (message `/Game/UserWork/c013265l/Interfaces/BPI_Interaction.I_Inspect` _helditem (`self.InteractingChar`)))))))

(event `/Game/UserWork/c013265l/Interfaces/BPI_Interaction.I_GiveItem`
  (params (ItemToGive :type "Actor Object Reference"))
  (set `self.HeldItem` ItemToGive))

(event `/Game/UserWork/c013265l/Interfaces/BPI_Interaction.I_RemoveItem`
  (set `self.HeldItem` null))

(event `/Game/UserWork/c013265l/Interfaces/BPI_Interaction.I_FreezeInput`
  (params (ShouldFreeze :type Boolean))
  (set `self.Should Freeze` ShouldFreeze))

(event `/Game/UserWork/c013265l/Interfaces/BPI_Interaction.I_DisableInput`
  (params (ShouldDisable :type Boolean))
  (bind _interactingchar (`self.InteractingChar`))
  (if ShouldDisable
    (`self.DisableInput` _interactingchar self)
    (else
      (`self.EnableInput` _interactingchar self))))

(event `InputAction|AttachPuzzlePiece`
  (params (Key :type "Key Structure"))
  (:`Pressed`
    (message `/Game/UserWork/c013265l/Interfaces/BPI_Interaction.I_AttachObject` (`self.HeldItem`))))

(event `InputAction|UIInteraction`
  (params (Key :type "Key Structure"))
  (:`Pressed`
    (message `/Game/UserWork/c013265l/Interfaces/BPI_Interaction.I_UiInteract` (`self.InteractingChar`) "None")))

(fn `GetCurrentMousePosition`
  (bind _returnvalue (`WidgetLayoutLibrary.GetMousePositionOnViewport`))
  (`|ExecutionSequence`
    (:`then_0`
      (message `/Game/UserWork/c013265l/Interfaces/BPI_WirePuzzle.I_CurrentMousePos` (`self.K2_GetPawn`) (`GameplayStatics.DeprojectScreenToWorld` self (`self.LastMousePosition`))))
    (:`then_1`
      (bind _output_get (set `self.LastMousePosition` _returnvalue)))))

(fn `UserConstructionScript`)