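; BP_Projector is an environmental projector that switches on when its referenced wire puzzle is completed.
; On BeginPlay it caches the intensities of its point and rect lights, binds TurnOn to the puzzle's completion event, then zeroes both lights.
; TurnOn restores the cached intensities and sets the material on the projector screen.
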(event `self.ReceiveBeginPlay`
  (set `self.PointLightIntensity` (`LightComponentBase.Intensity` (`self. `)))
  (set `self.RectLightIntensity` (`LightComponentBase.Intensity` (`self.RectLight`)))
  (add `/Game/c013265l/Puzzles/PCRoom/Blueprints/BP_WirePuzzleEnd.WirePuzzleComplete` (`self.PuzzleRef`) (delegate `TurnOn`))
  (`self.TurnOff`))

(event `TurnOff`
  (`LightComponent.SetIntensity` (`self. `) 0.0)
  (`LightComponent.SetIntensity` (`self.RectLight`) 0.0))

(event `TurnOn`
  (`LightComponent.SetIntensity` (`self. `) (`self.PointLightIntensity`))
  (`LightComponent.SetIntensity` (`self.RectLight`) (`self.RectLightIntensity`))
  (`/Game/s020301l/Blueprints/Environmental/BP_ProjectorScreen.SetMaterial` (`self.ProjectorScreen`)))

(fn `UserConstructionScript`)