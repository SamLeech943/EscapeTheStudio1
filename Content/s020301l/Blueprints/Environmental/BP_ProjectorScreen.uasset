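; BP_ProjectorScreen is an interactable projector screen that retracts and extends, and can switch its displayed material.
; When unlocked, IInteract flip-flops between playing and reversing a timeline that lerps the Cube's world Z scale from its captured start value to zero.
; A separate SetMaterial event flip-flops the Cube's material between colour bars and a default material, regardless of the lock.
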(event `/Game/c013265l/Interfaces/BPI_Interaction.I_Interact`
  (params (InteractingCharacter :type "/Game/s020301l/Blueprints/Character/BP_EscapeCharacter Object Reference") (InteractingWirePawn :type "/Game/c013265l/Puzzles/PCRoom/Blueprints/P_WirePuzzle Object Reference") (IsCrouched :type Boolean))
  (bind _cube (`self.Cube`))
  (bind _returnvalue (`SceneComponent.K2_GetComponentScale` _cube))
  (bind (_x _y) (`KismetMathLibrary.BreakVector3f` _returnvalue))
  (if (not (`self.IsLocked`))
    (`/Engine/EditorBlueprintResources/StandardMacros.FlipFlop`
      (:`A`
        (bind _output_get (set `self.StartScale` _returnvalue))
        (bind (_direction _newtrack_0) (`Timeline|ScaleMeDaddy` :!label _label)
          (:`Update`
            (`SceneComponent.SetWorldScale3D` _cube (`KismetMathLibrary.VLerp` _output_get (`KismetMathLibrary.MakeVector` _x _y) _newtrack_0)))))
      (:`B`
        (goto _label :!via `Reverse`)))))

(event `SetMaterial`
  (bind _cube (`self.Cube`))
  (`/Engine/EditorBlueprintResources/StandardMacros.FlipFlop`
    (:`A`
      (`PrimitiveComponent.SetMaterial` _cube 0 "/Game/s020301l/Materials/ImageMats/M_ColourBars.M_ColourBars"))
    (:`B`
      (`PrimitiveComponent.SetMaterial` _cube 0 "/Game/Assets/Materials/01_-_Default.01_-_Default"))))

(fn `UserConstructionScript`)