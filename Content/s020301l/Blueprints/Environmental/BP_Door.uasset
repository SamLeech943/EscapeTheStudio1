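; BP_Door is a lockable, interactable swinging door with a red or green light showing its lock state.
; Interacting while unlocked toggles it through a FlipFlop, with a Timeline driving the mesh yaw alongside open and close sounds.
; When flagged as part of a wire puzzle, it binds to puzzle completion, which unlocks and toggles it.
; SetLocked updates the light, while OpenDoor and CloseDoor bypass the lock and FlipFlop.
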(event `SetLocked`
  (params (`IsLocked?` :type Boolean))
  (set `self.locked` `IsLocked?`)
  (`self.ChangeMaterial`))

(event `self.ReceiveBeginPlay`
  (bind _doorlight (`self.DoorLight`))
  (if (`self.IsOnwirepuzzle`)
    (add `/Game/c013265l/Puzzles/PCRoom/Blueprints/BP_WirePuzzleEnd.WirePuzzleComplete` (`self.WirePuzzleEndRef`) (delegate `UnlockDoor`)))
  ;[1 1 1] At the beginning of the game it checks if the door is locked and sets the light properly
  (if (`self.locked`) :!label _label
    (`PrimitiveComponent.SetMaterial` _doorlight 0 "/Game/d016946l_Alex/Area_2_ComuterRoom/Lightswitch_NOT_USED/M_LightBox_RedEmergency.M_LightBox_RedEmergency")
    (else
      (`PrimitiveComponent.SetMaterial` _doorlight 0 "/Game/s020301l/Materials/M_GreenEmissive.M_GreenEmissive")
      (`GameplayStatics.PlaySound2D` "/Game/l014519/Audio/Door_Open/DoorOpen.DoorOpen" 1.0 1.0 0.0 null null))))

(event `ChangeMaterial`
  ;[1 1 1] At the beginning of the game it checks if the door is locked and sets the light properly
  (goto _label))

(event `UnlockDoor`
  (bind _returnvalue (`self.K2_GetActorLocation`))
  (set `self.locked` false)
  (`self.ChangeMaterial`)
  (`/Engine/EditorBlueprintResources/StandardMacros.FlipFlop` :!label _label_2
    (:`A`
      (`GameplayStatics.PlaySoundAtLocation` "/Game/Audio/could_use/interact/3maze_-__Doors__Locks_and_Drawers/door_open_004.door_open_004" _returnvalue (struct) 0.2 1.0 0.0 null null null null :!label _label_3)
      (bind (_direction _newtrack_0) (`Timeline|Timeline_0` :`NewTime` 0.0 :!label _label_4)
        (:`Update`
          (`SceneComponent.K2_SetRelativeRotation` (`self.Cube5`) (`KismetMathLibrary.MakeRotator` 0.0 0.0 _newtrack_0) false false))))
    (:`B`
      (`GameplayStatics.PlaySoundAtLocation` "/Game/Audio/could_use/interact/3maze_-__Doors__Locks_and_Drawers/door_close_003.door_close_003" _returnvalue (struct) 0.2 1.0 0.0 null null null null :!label _label_5)
      (goto _label_4 :!via `Reverse`))))

(event `/Game/c013265l/Interfaces/BPI_Interaction.I_Interact`
  (params (InteractingCharacter :type "/Game/s020301l/Blueprints/Character/BP_EscapeCharacter Object Reference") (InteractingWirePawn :type "/Game/c013265l/Puzzles/PCRoom/Blueprints/P_WirePuzzle Object Reference") (IsCrouched :type Boolean))
  (if (not (`self.locked`))
    (goto _label_2)))

(event `OpenDoor`
  (goto _label_3))

(event `CloseDoor`
  (goto _label_5))

(fn `UserConstructionScript`)