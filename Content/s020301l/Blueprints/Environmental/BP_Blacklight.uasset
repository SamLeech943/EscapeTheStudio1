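; Blacklight actor that reveals hidden footprints with a purple spotlight.
; Activate and Deactivate toggle the spotlight and holder emissive material through SetLight, swapping referenced footprints between glowing and invisible materials.
; It starts deactivated and binds an event to the referenced wire puzzle's completion.
; ChangeLightColour turns the lit lamp white and hides the footprints again.
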(event `self.ReceiveBeginPlay`
  (bind _puzzleendref (`self.PuzzleEndRef`))
  (`self.Deactivate`)
  (set `self.New Light Color` (struct :`R` 0.486275 :`B` 0.490196 :`A` 1.0))
  (set `self.LightEmisMat` "/Game/s020301l/Materials/M_PurpleEmissive.M_PurpleEmissive")
  (`/Engine/EditorBlueprintResources/StandardMacros.IsValid` _puzzleendref
    (:`Is Valid`
      (add `/Game/c013265l/Puzzles/PCRoom/Blueprints/BP_WirePuzzleEnd.WirePuzzleComplete` _puzzleendref (`|CreateDelegate` :!event `ChangeLightColour`)))))

(event `Activate`
  (`self.SetLight` true)
  (for _array_element (`self.FootprintArray`)
    (`PrimitiveComponent.SetMaterial` (`/Game/s020301l/Blueprints/Environmental/BP_Footprint.Plane` _array_element) 0 "/Game/s020301l/Images/M_FootprintGlow.M_FootprintGlow")))

(event `Deactivate`
  (`self.SetLight` false)
  (for _array_element (`self.FootprintArray`) :!label _label
    (`PrimitiveComponent.SetMaterial` (`/Game/s020301l/Blueprints/Environmental/BP_Footprint.Plane` _array_element) 0 "/Game/s020301l/Materials/M_Invisible.M_Invisible")))

(event `ChangeLightColour`
  (bind _output_get (set `self.New Light Color` (struct :`R` 1.0 :`G` 1.0 :`B` 1.0 :`A` 1.0)))
  (`LightComponent.SetLightColor` (`self.SpotLight`) _output_get true)
  (set `self.LightEmisMat` "/Game/s020301l/Materials/M_WhiteEmissive.M_WhiteEmissive")
  (`self.SetLight` true)
  (goto _label))

(fn `SetLight`
  (params (IsActive :type Boolean))
  (bind _holder1 (`self.Holder1`))
  (`SceneComponent.SetVisibility` (`self.SpotLight`) IsActive false)
  (if IsActive
    (`PrimitiveComponent.SetMaterial` _holder1 0 (`self.LightEmisMat`))
    (else
      (`PrimitiveComponent.SetMaterial` _holder1 0 "/Game/Maps/Modular_Pieces/Grey.Grey"))))

(fn `UserConstructionScript`)