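; BP_KeyDoor is a chained double door that unlocks and swings open once two BP_DoorKey actors are brought to it.
; A box overlap makes the carrier drop each key, destroys it and reveals a matching key mesh in a lock.
; The second key swaps locked chain, lock and key meshes for unlocked versions by toggling visibility, then a timeline rotates two hinges in opposite yaw directions.
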(event `self.ReceiveBeginPlay`
  (set `self.Increment` 0)
  (for _array_element (`|MakeArray` (`self.ChainUnlocked2`) (`self.Lock4`) (`self.Key4`) (`self.ChainUnlocked1`) (`self.Lock3`) (`self.Key3`) (`self.Key1`) (`self.Key2`))
    (`SceneComponent.SetVisibility` _array_element false false)))

(event `self.Box.OnComponentBeginOverlap`
  (params (OverlappedComponent :type "PrimitiveComponent Object Reference") (OtherActor :type "Actor Object Reference") (OtherComp :type "PrimitiveComponent Object Reference") (OtherBodyIndex :type Integer) (bFromSweep :type Boolean) (SweepResult :type "HitResult Structure (by ref)"))
  (bind _increment (`self.Increment`))
  (if (<= (`self.Increment`) 1)
    (bind _asbp_door_key (cast `/Game/s020301l/Blueprints/Environmental/BP_DoorKey` OtherActor))
    (`/Engine/EditorBlueprintResources/StandardMacros.IsValid` _asbp_door_key
      (:`Is Valid`
        (message `/Game/c013265l/Interfaces/BPI_Interaction.I_DropItem` _asbp_door_key (`/Game/c013265l/Interactables/BP_BaseInteractable.Interacting Character` _asbp_door_key))
        (`self.AttachKey` _asbp_door_key)
        (`/Engine/EditorBlueprintResources/StandardMacros.IncrementInt` _increment
          (:`  `
            (if (== _increment 2)
              (`self.UnlockDoor`)
              (bind (_direction _newtrack_0) (`Timeline|RotateMe`)
                (:`Update`
                  (`SceneComponent.K2_SetRelativeRotation` (`self.CringeHinge2`) (`KismetMathLibrary.MakeRotator` 0.0 0.0 _newtrack_0) false false)
                  (`SceneComponent.K2_SetRelativeRotation` (`self.CringeHinge1`) (`KismetMathLibrary.MakeRotator` 0.0 0.0 (* _newtrack_0 -1.0)) false false))))))))))

(fn `AttachKey`
  (params (NewParam :type "Actor Object Reference"))
  (`SceneComponent.SetVisibility` (`|GetArrayItem` (`|MakeArray` (`self.Key1`) (`self.Key2`)) (`self.Increment`)) true false)
  (`self.K2_DestroyActor` NewParam))

(fn `OpenDoor`
  (locals (NewLocalVar_0 :type "Rotator Structure" :default (struct))))

(fn `UnlockDoor`
  (for _array_element (`|MakeArray` (`self.ChainLocked`) (`self.Lock2`) (`self.Key2`) (`self.Lock1`) (`self.Key1`))
    (`SceneComponent.SetVisibility` _array_element false false))
  (for _array_element_2 (`|MakeArray` (`self.ChainUnlocked1`) (`self.Lock3`) (`self.Key3`) (`self.ChainUnlocked2`) (`self.Lock4`) (`self.Key4`))
    (`SceneComponent.SetVisibility` _array_element_2 true false)))

(fn `UserConstructionScript`)