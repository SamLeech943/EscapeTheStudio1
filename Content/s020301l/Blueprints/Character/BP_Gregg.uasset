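; BP_Gregg is a watcher character that alternates between looking around and reading a book, killing the player if spotted.
; A timeline rotates its Sphere during each search, then collision switches off for a short reading pause before a timer restarts the loop.
; When BP_EscapeCharacter overlaps the Capsule, a visibility trace checks line of sight.
; An unblocked trace stops the sweep, turns the spotlight red and calls SetDead after a brief delay.
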(event `self.ReceiveBeginPlay`
  ;[0.3308 0.5513 0.6979] Initialisation - S020301L
  (`self.LookAround`))

(event `LookAround`
  (bind _initialrotation (`self.InitialRotation`))
  ;[0.3308 0.5513 0.6979] Behaviour Loop - S020301L
  (if (not (`self.Found`))
    (set `self.IsSearching` true)
    (`self.SetActorEnableCollision` true)
    (set `self.InitialRotation` (`SceneComponent.K2_GetComponentRotation` (`self.Sphere`)))
    (bind (_direction _newtrack_0) (`Timeline|Timeline_0` :!via `PlayFromStart` :!label _label)
      (:`Update`
        (`SceneComponent.K2_SetWorldRotation` (`self.Sphere`) (`KismetMathLibrary.RLerp` _initialrotation (`KismetMathLibrary.ComposeRotators` _initialrotation (struct :`Yaw` -110.0)) _newtrack_0) false false))
      (:`Finished`
        (`self.ReadBook`)))))

(event `ReadBook`
  ;[0.3308 0.5513 0.6979] Behaviour Loop - S020301L
  (if (not (`self.Found`))
    (set `self.IsSearching` false)
    (`self.SetActorEnableCollision` false)
    (`KismetSystemLibrary.K2_SetTimerDelegate` (delegate `LookAround`) 2.0)
    (goto _label :!via `Stop`)))

(event `self.Capsule.OnComponentBeginOverlap`
  (params (OverlappedComponent :type "PrimitiveComponent Object Reference") (OtherActor :type "Actor Object Reference") (OtherComp :type "PrimitiveComponent Object Reference") (OtherBodyIndex :type Integer) (bFromSweep :type Boolean) (SweepResult :type "HitResult Structure (by ref)"))
  ;[0.3308 0.5513 0.6979] Detect Trigger - S020301L
  (bind _asbp_escape_character (cast `/Game/s020301l/Blueprints/Character/BP_EscapeCharacter` OtherActor))
  (bind _output_get (set `self.As BP Escape Character` _asbp_escape_character))
  (bind _outhit (`KismetSystemLibrary.LineTraceSingle` :`Start` (`SceneComponent.K2_GetComponentLocation` (`self.Sphere`)) :`End` (+ (`self.K2_GetActorLocation` _output_get) (0.0 0.0 15.0)) :`TraceChannel` "TraceTypeQuery1" :`DrawDebugType` "Persistent"))
  (if (not (`GameplayStatics.BreakHitResult` _outhit))
    (`self.IsFound`)))

(event `IsFound`
  (`|ExecutionSequence`
    (:`then_0`
      (goto _label :!via `Stop`))
    (:`then_1`
      (`/Engine/EditorBlueprintResources/StandardMacros.DoOnce` false
        (:`Completed`
          (set `self.Found` true)
          (`LightComponent.SetLightColor` (`self.SpotLight`) (struct :`R` 1.0 :`A` 1.0) true)
          (`KismetSystemLibrary.Delay` 0.4)
          (`/Game/s020301l/Blueprints/Character/BP_EscapeCharacter.SetDead` (`self.As BP Escape Character`)))))))

(fn `UserConstructionScript`)