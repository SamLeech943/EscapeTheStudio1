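; BP_LevelArea is a level trigger volume that starts the escape run when the player enters it.
; On the first overlap of its box by a BP_EscapeCharacter, it starts the player's timer.
; After a short delay it closes and locks the referenced start door behind the player, with a counter blocking repeat triggers.
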(event `self.Box.OnComponentBeginOverlap`
  (params (OverlappedComponent :type "PrimitiveComponent Object Reference") (OtherActor :type "Actor Object Reference") (OtherComp :type "PrimitiveComponent Object Reference") (OtherBodyIndex :type Integer) (bFromSweep :type Boolean) (SweepResult :type "HitResult Structure (by ref)"))
  (bind _startdoor (`self.StartDoor`))
  (bind _counter (`self.Counter`))
  (bind _asbp_escape_character (cast `/Game/s020301l/Blueprints/Character/BP_EscapeCharacter` OtherActor))
  (set `self.PlayerRef` _asbp_escape_character)
  (if (== 0 _counter)
    (`/Engine/EditorBlueprintResources/StandardMacros.IncrementInt` _counter
      (:`  `
        (`/Game/s020301l/Blueprints/Character/BP_EscapeCharacter.StartTimer` (`self.PlayerRef`))
        (`KismetSystemLibrary.Delay` 0.8)
        (`/Game/s020301l/Blueprints/Environmental/BP_Door.CloseDoor` _startdoor)
        (`/Game/s020301l/Blueprints/Environmental/BP_Door.SetLocked` _startdoor true)))))

(fn `UserConstructionScript`)