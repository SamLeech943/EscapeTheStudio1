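; BP_GameManager handles checkpoint respawning when the escape character dies.
; On BeginPlay it caches all BP_Checkpoint2 actors and the BP_EscapeCharacter, binds three handlers to the character's IsDead dispatcher, then initializes the character.
; The handlers select the active checkpoint with the highest index, move the player to it, and unload and reload that checkpoint's streamed level to reset it.
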(event `self.ReceiveBeginPlay`
  ;[0.1454 0.6395 0.6979] Game Manager - S020301L
  (bind _outactors (`GameplayStatics.GetAllActorsOfClass` "/Game/s020301l/Blueprints/System/BP_Checkpoint2.BP_Checkpoint2_C"))
  (bind _returnvalue (`GameplayStatics.GetActorOfClass` "/Game/s020301l/Blueprints/Character/BP_EscapeCharacter.BP_EscapeCharacter_C"))
  (set `self.Checkpoints` _outactors)
  (bind _output_get (set `self.PlayerCharRef` _returnvalue))
  (add `/Game/s020301l/Blueprints/Character/BP_EscapeCharacter.IsDead` _output_get (delegate `UpdateCheckpoint`))
  (add `/Game/s020301l/Blueprints/Character/BP_EscapeCharacter.IsDead` _output_get (delegate `ResetPlayer`))
  (add `/Game/s020301l/Blueprints/Character/BP_EscapeCharacter.IsDead` _output_get (delegate `RestartLevel`))
  (`/Game/s020301l/Blueprints/Character/BP_EscapeCharacter.Event Init` _output_get))

(event `UpdateCheckpoint`
  ;[0.1454 0.6395 0.6979] Game Manager - S020301L
  (for _array_element (`self.Checkpoints`)
    (if (`/Game/s020301l/Blueprints/System/BP_Checkpoint2.IsActive` _array_element)
      (if (>= (`/Game/s020301l/Blueprints/System/BP_Checkpoint2.CheckpointIndex` _array_element) (`self.CurrentIndex`))
        (bind _output_get (set `self.CurrentCheckpoint` _array_element))
        (set `self.CurrentIndex` (`/Game/s020301l/Blueprints/System/BP_Checkpoint2.CheckpointIndex` _output_get))))))

(event `ResetPlayer`
  ;[0.1454 0.6395 0.6979] Game Manager - S020301L
  (`self.K2_SetActorLocation` (`self.PlayerCharRef`) (`self.K2_GetActorLocation` (`self.CurrentCheckpoint`)) false false))

(event `RestartLevel`
  (bind _leveltoreset (`/Game/s020301l/Blueprints/System/BP_Checkpoint2.LevelToReset` (`self.CurrentCheckpoint`)))
  ;[0.1454 0.6395 0.6979] Game Manager - S020301L
  (`GameplayStatics.UnloadStreamLevel` _leveltoreset)
  (`GameplayStatics.LoadStreamLevel` _leveltoreset true)
  (`KismetSystemLibrary.PrintString` "Level Change"))

(fn `UserConstructionScript`)