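; Blacklight actor that reveals hidden footprints when switched on.
; Activate and Deactivate call SetLight to toggle the spotlight's visibility and swap the holder between emissive purple and grey.
; They also loop over FootprintArray, swapping each footprint's plane between green emissive and invisible materials, so the reveal ignores where the light points.
; It starts deactivated on BeginPlay.
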(event `self.ReceiveBeginPlay`
  (`self.Deactivate`))

(event `Activate`
  (`self.SetLight` true)
  (for _array_element (`self.FootprintArray`)
    (`PrimitiveComponent.SetMaterial` (`/Game/s020301l/Blueprints/BP_Footprint.Plane` _array_element) 0 "/Game/s020301l/Materials/M_GreenEmissive.M_GreenEmissive")))

(event `Deactivate`
  (`self.SetLight` false)
  (for _array_element (`self.FootprintArray`)
    (`PrimitiveComponent.SetMaterial` (`/Game/s020301l/Blueprints/BP_Footprint.Plane` _array_element) 0 "/Game/s020301l/Materials/M_Invisible.M_Invisible")))

(fn `SetLight`
  (params (IsActive :type Boolean))
  (bind _holder1 (`self.Holder1`))
  (`SceneComponent.SetVisibility` (`self.SpotLight`) IsActive false)
  (if IsActive
    (`PrimitiveComponent.SetMaterial` _holder1 0 "/Game/s020301l/Materials/M_PurpleEmissive.M_PurpleEmissive")
    (else
      (`PrimitiveComponent.SetMaterial` _holder1 0 "/Game/Maps/Modular_Pieces/Grey.Grey"))))

(fn `UserConstructionScript`)