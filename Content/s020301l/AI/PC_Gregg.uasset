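; AI controller for Gregg that starts the BT_Gregg behavior tree when it possesses a pawn.
; On possession it records the pawn's root rotation in the Blackboard as the start rotation.
; It also stores full and half rotation limits on either side of that start, built by combining fixed offsets with it, for use as Blackboard keys.
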(event `self.ReceivePossess`
  (params (PossessedPawn :type "Pawn Object Reference"))
  (bind _returnvalue (`AIBlueprintHelperLibrary.GetBlackboard` null))
  (bind _returnvalue_2 (`SceneComponent.K2_GetComponentRotation` (`Actor.RootComponent` PossessedPawn)))
  (`self.RunBehaviorTree` "/Game/s020301l/AI/BT_Gregg.BT_Gregg")
  (`BlackboardComponent.SetValueAsRotator` _returnvalue "StartRotation" _returnvalue_2)
  (`BlackboardComponent.SetValueAsRotator` _returnvalue "MaxRotation" (`KismetMathLibrary.ComposeRotators` _returnvalue_2 (struct :`Yaw` 90.0)))
  (`BlackboardComponent.SetValueAsRotator` _returnvalue "MinRotation" (`KismetMathLibrary.ComposeRotators` _returnvalue_2 (struct :`Yaw` -90.0)))
  (`BlackboardComponent.SetValueAsRotator` _returnvalue "HalfMaxRotation" (`KismetMathLibrary.ComposeRotators` _returnvalue_2 (struct :`Yaw` 45.0)))
  (`BlackboardComponent.SetValueAsRotator` _returnvalue "HalfMinRotation" (`KismetMathLibrary.ComposeRotators` _returnvalue_2 (struct :`Yaw` -45.0))))

(fn `UserConstructionScript`)