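; BP_DoubleDoor is a lockable double door that swings open when interacted with.
; The DoorOpening timeline rotates the right hinge and left door in mirrored yaw and turns the left handle.
; Interaction plays the timeline only when unlocked, while OpenDoor and CloseDoor play or reverse it without checking the lock.
; UnlockDoor writes its Lock argument straight into IsLocked, so it can also lock the door.
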(event `OpenDoor`
  (bind (_direction _doorrot _handleturn) (`Timeline|DoorOpening` :!label _label)
    (:`Update`
      (`SceneComponent.K2_SetRelativeRotation` (`self.DoorRHinge`) (`KismetMathLibrary.MakeRotator` 0.0 0.0 _doorrot) false false)
      (`SceneComponent.K2_SetRelativeRotation` (`self.DoorL`) (`KismetMathLibrary.MakeRotator` 0.0 0.0 (* _doorrot -1.0)) false false)
      (`SceneComponent.K2_SetRelativeRotation` (`self.DoorHandleL`) (`KismetMathLibrary.MakeRotator` 0.0 (* _handleturn -1.0) 180.0) false false))))

(event `/Game/c013265l/Interfaces/BPI_Interaction.I_Interact`
  (params (InteractingCharacter :type "/Game/s020301l/Blueprints/Character/BP_EscapeCharacter Object Reference") (InteractingWirePawn :type "/Game/c013265l/Puzzles/PCRoom/Blueprints/P_WirePuzzle Object Reference") (IsCrouched :type Boolean))
  (if (not (`self.IsLocked`))
    (goto _label)))

(event `CloseDoor`
  (goto _label :!via `Reverse`))

(event `UnlockDoor`
  (params (`Lock?` :type Boolean))
  (set `self.IsLocked` `Lock?`))

(fn `UserConstructionScript`)