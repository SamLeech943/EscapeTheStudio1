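; A spotlight actor that flickers and plays an ambient electrical hum.
; On BeginPlay it caches the starting intensities of its SpotLight and RectLight and spawns the hum sound at its location with ambience attenuation.
; A timeline then drives both lights by multiplying each cached intensity by the same flicker curve, so they flicker in sync relative to their placed brightness.
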(event `self.ReceiveBeginPlay`
  (set `self.SpotlightIntensity` (`LightComponentBase.Intensity` (`self.SpotLight`)))
  (set `self.RectLightIntensity` (`LightComponentBase.Intensity` (`self.RectLight`)))
  (`GameplayStatics.SpawnSoundAtLocation` "/Game/Audio/Cues/Ambience/Ambience_LightHum.Ambience_LightHum" (`self.K2_GetActorLocation`) (struct) (`self.Volume Multiplier`) 1.0 0.0 "/Game/Audio/Cues/DefaultAttenuations/SA_DefaultAmbience.SA_DefaultAmbience" null)
  (bind (_direction _flicker1) (`Timeline|FlickerTimeline`)
    (:`Update`
      (`LightComponent.SetIntensity` (`self.SpotLight`) (* _flicker1 (`self.SpotlightIntensity`)))
      (`LightComponent.SetIntensity` (`self.RectLight`) (* _flicker1 (`self.RectLightIntensity`))))))

(fn `UserConstructionScript`)