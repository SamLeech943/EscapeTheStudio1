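; Player controller for an escape room game that handles the Interact and Inspect inputs.
; Interact runs a Visibility line trace and, if the hit actor implements BPI_Interact, stores it as the current object, sends it the interact message and resets inspect mode.
; Inspect toggles the InspectMode flag once an object is held; this graph only sets that flag and never clears HasObject.
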(event `self.ReceiveBeginPlay`
  (set `self.PlayerCharacter` (`self.K2_GetPawn`)))

(event `InputAction|Interect`
  (params (Key :type "Key Structure"))
  (:`Pressed`
    (bind (_outhit _returnvalue) (`KismetSystemLibrary.LineTraceSingle` (0.0 0.0 0.0) (0.0 0.0 0.0) "TraceTypeQuery1"))
    (if _returnvalue
      (bind (_bblockinghit _binitialoverlap _time _distance _location _impactpoint _normal _impactnormal _physmat _hitactor) (`GameplayStatics.BreakHitResult` _outhit))
      (if (`KismetSystemLibrary.DoesImplementInterface` _hitactor "/Game/c013265l/Interfaces/BPI_Interact.BPI_Interact_C")
        (bind _output_get (set `self.CurrentObject` _hitactor))
        (message `/Game/c013265l/Interfaces/BPI_Interact.I_Interact` _output_get)
        (set `self.HasObject` true)
        (set `self.InspectMode` false)))))

(event `InputAction|Inspect`
  (params (Key :type "Key Structure"))
  (:`Pressed`
    (if (`self.HasObject`)
      (if (`self.InspectMode`)
        (set `self.InspectMode` false)
        (else
          (set `self.InspectMode` true))))))

(fn `UserConstructionScript`)