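; BP_AmbientSoundPlayer schedules random ambient sounds with pauses between them.
; A timer started at BeginPlay calls PlayRandomAmbience, passing Type, IsRandom and itself as sound manager, then clears itself.
; IAmbienceFinished picks a new random delay and restarts the timer, so each gap begins once playback reports completion.
; An unconnected leftover chain plays a creepy drone directly with fades.
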(event `/Game/c013265l/Interfaces/BPI_Music.I_AmbienceFinished`
  ;[0 0.2865 0.00931] c013265l - Set Time between ambience
  (set `self.TimeBetweenAmbience` (`KismetMathLibrary.RandomFloatInRange` 15.0 35.0))
  (bind _returnvalue (`KismetSystemLibrary.K2_SetTimerDelegate` (delegate `PlayAmbience`) (`self.TimeBetweenAmbience`) true :!label _label))
  (set `self.AmbienceHandle` _returnvalue))

(event `self.ReceiveBeginPlay`
  ;[0 0.2865 0.00931] c013265l - Set Time between ambience
  (goto _label))

(event `PlayAmbience`
  (`self.PlayRandomAmbience` (`self.Type`) (`self.Is Random`) self)
  (`KismetSystemLibrary.K2_ClearAndInvalidateTimerHandle` (`self.AmbienceHandle`)))

(fn `UserConstructionScript`)