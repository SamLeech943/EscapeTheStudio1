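; Trigger volume that starts rain and recurring thunder ambience at a target actor's location.
; Once enabled by SoundCanPlay, a BP_EscapeCharacter overlapping the box spawns pitched-down rain with a fade-in and starts the thunder timer.
; Each thunder clap clears and restarts the timer with a new random delay.
; ClearRainSound fades and destroys the rain component, leaving the thunder timer untouched.
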(event `ClearRainSound`
  (bind _rainsound (`self.RainSound`))
  ;[0 0.2708 0.02237] c013265l - Clear Sound
  (`AudioComponent.FadeOut` _rainsound 3.0 0.0 "Linear")
  (`ActorComponent.K2_DestroyComponent` _rainsound))

(event `SoundCanPlay`
  (set `self.CanPlay` true))

(event `StartThunderTimer`
  ;[0 0.2708 0.02237] c013265l - Spawn rain and thunder
  (set `self.TimeBetweenThunder` (`KismetMathLibrary.RandomFloatInRange` 12.0 22.0))
  (bind _returnvalue (`KismetSystemLibrary.K2_SetTimerDelegate` (delegate `PlayThunder`) (`self.TimeBetweenThunder`) true :!label _label))
  (set `self.ThunderHandle` _returnvalue))

(event `self.Box.OnComponentBeginOverlap`
  (params (OverlappedComponent :type "PrimitiveComponent Object Reference") (OtherActor :type "Actor Object Reference") (OtherComp :type "PrimitiveComponent Object Reference") (OtherBodyIndex :type Integer) (bFromSweep :type Boolean) (SweepResult :type "HitResult Structure (by ref)"))
  ;[0 0.2708 0.02237] c013265l - Spawn rain and thunder
  (if (`self.CanPlay`)
    (cast `/Game/s020301l/Blueprints/Character/BP_EscapeCharacter` OtherActor)
    (if (`self.SingleUse`)
      (`/Engine/EditorBlueprintResources/StandardMacros.DoOnce` false
        (:`Completed`
          _)))
    (bind _returnvalue (`GameplayStatics.SpawnSoundAtLocation` (`self.SoundToPlay`) (`self.K2_GetActorLocation` (`self.ActorToPlaySoundAt`)) (struct) 1.0 0.6 0.0 null null))
    (bind _output_get (set `self.RainSound` _returnvalue))
    (`AudioComponent.FadeIn` _output_get 3.0 1.0 0.0 "SCurve")
    (goto _label)))

(event `PlayThunder`
  ;[0 0.2708 0.02237] c013265l - Spawn rain and thunder
  (`GameplayStatics.PlaySoundAtLocation` "/Game/Audio/Usable_Sound_Effects/Usable_Sound_Effects/Ambient_noise/Thunder_SC.Thunder_SC" (`self.K2_GetActorLocation` (`self.ActorToPlaySoundAt`)) (struct) 1.0 1.0 0.0 null null null null)
  (`KismetSystemLibrary.K2_ClearAndInvalidateTimerHandle` (`self.ThunderHandle`))
  (`self.StartThunderTimer`))

(fn `UserConstructionScript`)