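; BP_CollisionSoundPlayer is an audio trigger that plays a sound once when the player walks into its box after a wire puzzle is completed.
; On BeginPlay it binds an event to the referenced wire puzzle end's completion, with AllowSoundToPlay available to set the CanPlay gate.
; A box overlap by BP_EscapeCharacter then passes a DoOnce and plays the configured sound at a chosen actor's location.
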(event `self.ReceiveBeginPlay`
  (add `/Game/c013265l/Puzzles/PCRoom/Blueprints/BP_WirePuzzleEnd.WirePuzzleComplete` (`self.WirePuzzleEndRef`) (`|CreateDelegate` :!event `AllowSoundToPlay`)))

(event `AllowSoundToPlay`
  (set `self.CanPlay` true))

(event `self.Box.OnComponentBeginOverlap`
  (params (OverlappedComponent :type "PrimitiveComponent Object Reference") (OtherActor :type "Actor Object Reference") (OtherComp :type "PrimitiveComponent Object Reference") (OtherBodyIndex :type Integer) (bFromSweep :type Boolean) (SweepResult :type "HitResult Structure (by ref)"))
  (if (`self.CanPlay`)
    (cast `/Game/s020301l/Blueprints/Character/BP_EscapeCharacter` OtherActor)
    (`/Engine/EditorBlueprintResources/StandardMacros.DoOnce` false
      (:`Completed`
        (`GameplayStatics.PlaySoundAtLocation` (`self.SoundToPlay`) (`self.K2_GetActorLocation` (`self.ActorToPlaySoundAt`)) (struct) 1.0 1.0 0.0 null null null null)))))

(fn `UserConstructionScript`)