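; Base interactable actor for physics items that a character can pick up, drop and inspect.
; Pickup plays a sound, disables physics, lerps the mesh to the character's ItemHoldPoint, attaches it and sets walk speed.
; Inspection freezes player input, slides the item toward the camera and enables left-drag rotation, then reverses the same timeline to reattach it.
; Interface messages notify the player controller, while DoOnce gates block repeated pickup or inspection.
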(event `/Game/c013265l/Interfaces/BPI_Interaction.I_Interact`
  (params (InteractingCharacter :type "/Game/s020301l/Blueprints/Character/BP_EscapeCharacter Object Reference") (InteractingWirePawn :type "/Game/c013265l/Puzzles/PCRoom/Blueprints/P_WirePuzzle Object Reference") (IsCrouched :type Boolean))
  (bind _itemholdpoint (`/Game/s020301l/Blueprints/Character/BP_EscapeCharacter.ItemHoldPoint` (`self.Interacting Character`)))
  (`/Engine/EditorBlueprintResources/StandardMacros.DoOnce` false :!label _label
    (:`Completed`
      (`GameplayStatics.PlaySoundAtLocation` (`self.PickupSound`) (`self.K2_GetActorLocation`) (struct) 0.5 1.0 (`self.PickupSoundStartTime`) "/Game/Audio/Cues/DefaultAttenuations/SA_DefaultPickup.SA_DefaultPickup" null null null)
      (set `self.Interacting Character` InteractingCharacter)
      ;[0.01096 0.2346 0.004391] Pick up item
      (`PrimitiveComponent.IgnoreActorWhenMoving` (`self.Mesh`) (`self.Interacting Character`) true)
      (`PrimitiveComponent.SetSimulatePhysics` (`self.Mesh`) false)
      (bind (_direction _alpha) (`Timeline|StartSmoothMovement`)
        (:`Update`
          (`self.K2_SetActorLocation` (`KismetMathLibrary.VLerp` (`self.K2_GetActorLocation`) (`SceneComponent.K2_GetComponentLocation` _itemholdpoint) _alpha)))
        (:`Finished`
          (`self.K2_AttachToComponent` self _itemholdpoint "None" "SnapToTarget" "SnapToTarget" "KeepWorld" true)
          (message `/Game/c013265l/Interfaces/BPI_Interaction.I_IsPickedUp` (`GameplayStatics.GetPlayerController` 0))
          (set `/Game/s020301l/Blueprints/Character/BP_EscapeCharacter.WalkSpeed` (`self.Char Speed`) (`self.Interacting Character`)))))))

(event `ResetInteract`
  (goto _label :!via `Reset`))

(event `/Game/c013265l/Interfaces/BPI_Interaction.I_DropItem`
  (params (OwningChar :type "/Game/s020301l/Blueprints/Character/BP_EscapeCharacter Object Reference"))
  ;[0.01096 0.2346 0.004391] Drop item
  (`self.K2_DetachFromActor` "KeepWorld" "KeepWorld" "KeepWorld")
  (`PrimitiveComponent.SetSimulatePhysics` (`self.Mesh`) true)
  (message `/Game/c013265l/Interfaces/BPI_Interaction.I_IsDropped` (`GameplayStatics.GetPlayerController` 0))
  (`PrimitiveComponent.IgnoreActorWhenMoving` (`self.Mesh`) (`self.Interacting Character`) false)
  (set `self.Interacting Character` null)
  (`self.ResetInteract`))

(event `/Game/c013265l/Interfaces/BPI_Interaction.I_Inspect`
  (params (InspectingChar :type "/Game/s020301l/Blueprints/Character/BP_EscapeCharacter Object Reference"))
  (bind _returnvalue (`GameplayStatics.GetPlayerController` 0))
  (bind _returnvalue_2 (`GameplayStatics.GetPlayerController` 0))
  (bind _returnvalue_3 (`SceneComponent.K2_GetComponentLocation` (`self.Mesh`)))
  ;[0.01096 0.2346 0.004391] Start/Stop inspection
  (`/Engine/EditorBlueprintResources/StandardMacros.DoOnce` false :!label _label_2
    (:`Completed`
      (message `/Game/c013265l/Interfaces/BPI_Interaction.I_FreezeInput` _returnvalue true)
      (message `/Game/c013265l/Interfaces/BPI_Interaction.I_FreezeInput` (`Controller.K2_GetPawn` _returnvalue) true)
      (set `self.StartInspectLoc` _returnvalue_3)
      (set `self.TargetInspectLoc` (+ _returnvalue_3 (* (`SceneComponent.GetForwardVector` (`PlayerCameraManager.TransformComponent` (`GameplayStatics.GetPlayerCameraManager` 0))) -30.0)))
      (set `self.CanDrop` false)
      (`|ExecutionSequence`
        (:`then_0`
          (set `PlayerController.bShowMouseCursor` true _returnvalue_2))
        (:`then_1`
          (`self.EnableInput` _returnvalue_2)
          (bind (_direction _alpha) (`Timeline|MoveToInspect` :!label _label_3)
            (:`Update`
              (`self.K2_SetActorLocation` (`KismetMathLibrary.VLerp` (`self.StartInspectLoc`) (`self.TargetInspectLoc`) _alpha)))
            (:`Finished`
              (switch `ETimelineDirection` _direction
                (:`Forward`
                  (set `self.CanRotate` true))
                (:`Backward`
                  (`self.ResetInspect`))))))))))

(event `ResetInspect`
  (bind _returnvalue (`GameplayStatics.GetPlayerController` 0))
  ;[0.01096 0.2346 0.004391] Start/Stop inspection
  (`self.K2_AttachToComponent` self (`/Game/s020301l/Blueprints/Character/BP_EscapeCharacter.ItemHoldPoint` (`self.Interacting Character`)) "None" "SnapToTarget" "SnapToTarget" "KeepWorld" true)
  (set `PlayerController.bShowMouseCursor` false _returnvalue)
  (message `/Game/c013265l/Interfaces/BPI_Interaction.I_FreezeInput` _returnvalue false)
  (message `/Game/c013265l/Interfaces/BPI_Interaction.I_FreezeInput` (`Controller.K2_GetPawn` _returnvalue) false)
  (goto _label_2 :!via `Reset`))

(event `ReverseItemMovement`
  ;[0.01096 0.2346 0.004391] Start/Stop inspection
  (goto _label_3 :!via `Reverse`))

(event `/Game/c013265l/Interfaces/BPI_Interaction.I_StopInspecting`
  ;[0.01096 0.2346 0.004391] Start/Stop inspection
  (`self.DisableInput` (`GameplayStatics.GetPlayerController` 0))
  (set `self.CanRotate` false)
  (`self.K2_DetachFromActor` "KeepWorld" "KeepWorld" "KeepWorld")
  (`self.ReverseItemMovement`))

(event `InputAxisKey|MouseX`
  (params (AxisValue :type "Float (single-precision)"))
  ;[0.01096 0.2346 0.004391] Rotate item with mouse
  (if (`self.IsRotating`)
    (`self.K2_SetActorRotation` (`KismetMathLibrary.ComposeRotators` (`self.K2_GetActorRotation`) (`KismetMathLibrary.MakeRotator` 0.0 0.0 (* AxisValue -5.0))))))

(event `Key|LeftMouseButton`
  (params (Key :type "Key Structure"))
  ;[0.01096 0.2346 0.004391] Rotate item with mouse
  (:`Pressed`
    (if (`self.CanRotate`)
      (set `self.IsRotating` true)))
  (:`Released`
    (set `self.IsRotating` false)))

(event `InputAxisKey|MouseY`
  (params (AxisValue :type "Float (single-precision)"))
  ;[0.01096 0.2346 0.004391] Rotate item with mouse
  (if (`self.IsRotating`)
    (`self.K2_SetActorRotation` (`KismetMathLibrary.ComposeRotators` (`self.K2_GetActorRotation`) (`KismetMathLibrary.MakeRotator` 0.0 (* AxisValue -5.0))))))

(fn `UserConstructionScript`
  (`PrimitiveComponent.SetSimulatePhysics` (`self.Mesh`) (`self.HasPhysics`)))