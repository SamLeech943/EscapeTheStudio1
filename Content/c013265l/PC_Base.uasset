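; Base player controller for an escape game that handles picking up, inspecting and dropping items and creates the player HUD.
; Interact, while empty-handed, line-traces from the first-person camera and messages hit actors implementing BPI_Interaction, storing them as the held item.
; Inspect toggles inspection and DropItem releases the item unless input is frozen, both through interface messages.
; Pickup and drop callbacks update the held state and crosshair visibility.
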(event `self.ReceiveBeginPlay`
  (bind _asbp_escape_character (cast `/Game/s020301l/Blueprints/BP_EscapeCharacter` (`self.K2_GetPawn`)))
  (set `self.InteractingChar` _asbp_escape_character)
  (bind _returnvalue (`|CreateWidget` "/Game/A018745l/UI/Player_UI.Player_UI_C" self))
  (bind _output_get (set `self.Player UI` _returnvalue))
  (`UserWidget.AddToViewport` _output_get 0))

(event `InputAction|Interact`
  (params (Key :type "Key Structure"))
  (bind _firstpersoncamera (`/Game/s020301l/Blueprints/BP_EscapeCharacter.FirstPersonCamera` (`self.InteractingChar`)))
  (bind _returnvalue (`SceneComponent.K2_GetComponentLocation` _firstpersoncamera))
  (:`Pressed`
    (if (not (`self.HasItem`))
      (bind (_outhit _returnvalue_2) (`KismetSystemLibrary.LineTraceSingleForObjects` :`Start` _returnvalue :`End` (+ _returnvalue (* (`KismetMathLibrary.GetForwardVector` (`SceneComponent.K2_GetComponentRotation` _firstpersoncamera)) 500.0)) :`ObjectTypes` (`|MakeArray` "ObjectTypeQuery8" :!type "EObjectTypeQuery Enum") :`DrawDebugType` "ForDuration"))
      (if _returnvalue_2
        (bind (_bblockinghit _binitialoverlap _time _distance _location _impactpoint _normal _impactnormal _physmat _hitactor) (`GameplayStatics.BreakHitResult` _outhit))
        (if (`KismetSystemLibrary.DoesImplementInterface` _hitactor "/Game/c013265l/Interfaces/BPI_Interaction.BPI_Interaction_C")
          (bind _output_get (set `self.HeldItem` _hitactor))
          (message `/Game/c013265l/Interfaces/BPI_Interaction.I_Interact` _output_get (`self.InteractingChar`))
          (set `self.IsInspecting` false))))))

(event `/Game/c013265l/Interfaces/BPI_Interaction.I_IsDropped`
  (set `self.HasItem` false)
  (`Widget.SetVisibility` (`/Game/A018745l/UI/Player_UI.Crosshair` (`self.Player UI`)) "Visible"))

(event `/Game/c013265l/Interfaces/BPI_Interaction.I_IsPickedUp`
  (set `self.HasItem` true)
  (`Widget.SetVisibility` (`/Game/A018745l/UI/Player_UI.Crosshair` (`self.Player UI`)) "Hidden"))

(event `InputAction|DropItem`
  (params (Key :type "Key Structure"))
  (:`Pressed`
    (if (`self.Should Freeze`)
      _
      (elif (`self.HasItem`)
        (message `/Game/c013265l/Interfaces/BPI_Interaction.I_DropItem` (`self.HeldItem`) (`self.InteractingChar`))))))

(event `InputAction|Inspect`
  (params (Key :type "Key Structure"))
  (bind _helditem (`self.HeldItem`))
  (:`Pressed`
    (if (`self.HasItem`)
      (if (`self.IsInspecting`)
        (set `self.IsInspecting` false)
        (message `/Game/c013265l/Interfaces/BPI_Interaction.I_StopInspecting` _helditem)
        (else
          (set `self.IsInspecting` true)
          (message `/Game/c013265l/Interfaces/BPI_Interaction.I_Inspect` _helditem (`self.InteractingChar`)))))))

(event `/Game/c013265l/Interfaces/BPI_Interaction.I_FreezeInput`
  (params (ShouldFreeze :type Boolean))
  (set `self.Should Freeze` ShouldFreeze))

(fn `UserConstructionScript`)