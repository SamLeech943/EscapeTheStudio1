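; Controller actor for the PC room wire puzzle, housed behind a hinged door.
; On interact it freezes the character, swings the door open on a timeline, then possesses a wire pawn; exiting restores the character and reverses the door.
; Interface messages start voltage from the starting wire and toggle wire slot collision as wires attach or detach.
; It binds to the puzzle end's completion event, with a handler that turns the grid green.
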(event `self.ReceiveBeginPlay`
  (bind _puzzleendref (`self.PuzzleEndRef`))
  (`/Engine/EditorBlueprintResources/StandardMacros.IsValid` _puzzleendref
    (:`Is Valid`
      (add `/Game/c013265l/Puzzles/PCRoom/Blueprints/BP_WirePuzzleEnd.WirePuzzleComplete` _puzzleendref (`|CreateDelegate` :!event `WirePuzzleFinished`)))))

(event `/Game/c013265l/Interfaces/BPI_WirePuzzle.I_SendVoltage`
  (message `/Game/c013265l/Interfaces/BPI_WirePuzzle.I_WireConnected` (`self.StartingWire`) 0 null))

(event `WirePuzzleFinished`
  (`PrimitiveComponent.SetMaterial` (`self.Grid`) 1 "/Game/s020301l/Materials/M_GreenEmissive.M_GreenEmissive"))

(event `/Game/c013265l/Interfaces/BPI_Interaction.I_Interact`
  (params (InteractingCharacter :type "/Game/s020301l/Blueprints/Character/BP_EscapeCharacter Object Reference") (InteractingWirePawn :type "/Game/c013265l/Puzzles/PCRoom/Blueprints/P_WirePuzzle Object Reference"))
  (bind _returnvalue (`GameplayStatics.GetPlayerController` 0))
  (bind _output_get (set `self.Interacting Character` InteractingCharacter))
  (message `/Game/c013265l/Interfaces/BPI_Interaction.I_FreezeInput` _output_get true)
  (bind (_direction _angle) (`Timeline|DoorOpening` :!label _label)
    (:`Update`
      (`SceneComponent.K2_SetRelativeRotation` (`self.Door`) (`KismetMathLibrary.MakeRotator` 0.0 0.0 _angle) false false))
    (:`Finished`
      (switch `ETimelineDirection` _direction
        (:`Forward`
          (`Controller.Possess` (`GameplayStatics.GetPlayerController` 0) (`self.PawnRef`))
          (message `/Game/c013265l/Interfaces/BPI_WirePuzzle.I_SwitchToWirePawn` (`self.PawnRef`) self)
          (message `/Game/c013265l/Interfaces/BPI_Interaction.I_IsPickedUp` _returnvalue)
          (message `/Game/c013265l/Interfaces/BPI_Interaction.I_DisableInput` _returnvalue true))))))

(event `/Game/c013265l/Interfaces/BPI_WirePuzzle.I_ExitWirePuzzle`
  (bind _returnvalue (`GameplayStatics.GetPlayerController` 0))
  (bind _interacting_character (`self.Interacting Character`))
  (`Controller.Possess` _returnvalue _interacting_character)
  (message `/Game/c013265l/Interfaces/BPI_Interaction.I_FreezeInput` _interacting_character false)
  (message `/Game/c013265l/Interfaces/BPI_Interaction.I_IsDropped` _returnvalue)
  (message `/Game/c013265l/Interfaces/BPI_Interaction.I_DisableInput` _returnvalue false)
  (goto _label :!via `Reverse`))

(event `/Game/c013265l/Interfaces/BPI_WirePuzzle.I_WireAttached`
  (params (WireSlot :type "PrimitiveComponent Object Reference"))
  (`PrimitiveComponent.SetCollisionEnabled` WireSlot "NoCollision"))

(event `/Game/c013265l/Interfaces/BPI_WirePuzzle.I_WireUnattached`
  (params (CurrentWireSlot :type "PrimitiveComponent Object Reference"))
  (`PrimitiveComponent.SetCollisionEnabled` CurrentWireSlot "QueryOnly"))

(fn `UserConstructionScript`)